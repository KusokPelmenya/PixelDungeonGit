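; GM_Base is a base game mode that tracks living enemies and picks a random level.
; RegisterEnemy and UnregisterEnemy maintain the AliveEnemies count; when it drops to zero or below, the level is flagged cleared, "Done!" is printed and OnLevelCleared is broadcast.
; GetRandomLevel permanently removes the last level name from the available list, then stores a random pick as the new last level, without loading it.
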(fn `GetRandomLevel`
  (bind _availblelevels (`self.AvailbleLevels`))
  (`KismetArrayLibrary.Array_RemoveItem` _availblelevels (`self.LastLevelName`))
  (bind _output_get (set `self.ChosenLevel` (`KismetArrayLibrary.Array_Random` _availblelevels)))
  (set `self.LastLevelName` _output_get))

(fn `RegisterEnemy`
  (bind _result (`/Engine/EditorBlueprintResources/StandardMacros.IncrementInt` (`self.AliveEnemies`))
    (:`  `
      (set `self.AliveEnemies` _result))))

(fn `UnregisterEnemy`
  (bind _result (`/Engine/EditorBlueprintResources/StandardMacros.DecrementInt` (`self.AliveEnemies`))
    (:`  `
      (bind _output_get (set `self.AliveEnemies` _result))
      (if (<= _output_get 0)
        (set `self.bLevelCleared` true)
        (`KismetSystemLibrary.PrintString` "Done!")
        (`self.OnLevelCleared`)))))

(fn `UserConstructionScript`)