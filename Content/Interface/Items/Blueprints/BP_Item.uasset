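; BP_Item is a world item that the BP_GG player character can pick up, displayed as a sprite.
; InitItem stores a row name and sets the sprite from that row's image in InventoryDatatable_T.
; Sphere overlap begin and end set or clear the player's CanBePickedUp flag and CurrentItem reference.
; The overlap handlers fetch player 0 directly without checking which actor overlapped.
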(event `Init Item`
  (params (`Row Name` :type Name))
  (bind _output_get (set `self.Row Name` `Row Name`))
  (bind _returnvalue (`|GetDataTableRow` "/Game/Interface/Craft_Menu/Crafting_window/BluePrints/InventoryDatatable_T.InventoryDatatable_T" _output_get)
    (:`then`
      (`PaperSpriteComponent.SetSprite` (`self.Item_Sprite`) (`.Image_43_6540FF4942EF788004B81CA9DDEE4CAB` (break `/Game/Interface/Craft_Menu/Crafting_window/BluePrints/Item_T` _returnvalue))))))

(event `self.Sphere.OnComponentBeginOverlap`
  (params (OverlappedComponent :type "PrimitiveComponent Object Reference") (OtherActor :type "Actor Object Reference") (OtherComp :type "PrimitiveComponent Object Reference") (OtherBodyIndex :type Integer) (bFromSweep :type Boolean) (SweepResult :type "HitResult Structure (by ref)"))
  (bind _asbp_gg (cast `/Game/character/Blueprint/BP_GG` (`GameplayStatics.GetPlayerCharacter` 0)))
  (set `/Game/character/Blueprint/BP_GG.CanBePickedUp` true _asbp_gg)
  (set `/Game/character/Blueprint/BP_GG.CurrentItem` self _asbp_gg))

(event `self.Sphere.OnComponentEndOverlap`
  (params (OverlappedComponent :type "PrimitiveComponent Object Reference") (OtherActor :type "Actor Object Reference") (OtherComp :type "PrimitiveComponent Object Reference") (OtherBodyIndex :type Integer))
  (bind _asbp_gg (cast `/Game/character/Blueprint/BP_GG` (`GameplayStatics.GetPlayerCharacter` 0)))
  (set `/Game/character/Blueprint/BP_GG.CanBePickedUp` false _asbp_gg)
  (set `/Game/character/Blueprint/BP_GG.CurrentItem` null _asbp_gg))

(fn `UserConstructionScript`)