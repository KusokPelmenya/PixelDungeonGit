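; Enemy actor with a health pool and an attached HP bar widget, destroyed when its health runs out.
; On BeginPlay it fills current HP from the max value and sets itself as the Target of the TEST_V_HPBar_rarely widget.
; AnyDamage prints a debug string, subtracts the damage from HP and destroys the actor at zero or below.
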(event `self.ReceiveBeginPlay`
  (set `self.ft_HP` (`self.fl_maxHP`))
  (bind _astest_v_hpbar_rarely (cast `/Game/enemy/HP_bar/HP_bar_rarely/TEST_V_HPBar_rarely` (`WidgetComponent.GetWidget` (`self.HP_Bar`))))
  (set `/Game/enemy/HP_bar/HP_bar_rarely/TEST_V_HPBar_rarely.Target` self _astest_v_hpbar_rarely))

(event `self.ReceiveAnyDamage`
  (params (Damage :type "Float (single-precision)") (DamageType :type "DamageType Object Reference") (InstigatedBy :type "Controller Object Reference") (DamageCauser :type "Actor Object Reference"))
  (`KismetSystemLibrary.PrintString` "Hello")
  (bind _output_get (set `self.ft_HP` (- (`self.ft_HP`) Damage)))
  (if (<= _output_get 0.0)
    (`self.K2_DestroyActor`)))

(fn `UserConstructionScript`)