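; Enemy spawner that fills a level at BeginPlay by spending a LevelDifficulty budget on enemies from EnemyPool.
; While budget remains, each affordable pool entry joins AvailableEnemies, which is never cleared, and triggers a spawn at a random SpawnPoints location.
; Spawned class and deducted cost use separate random picks from that list, so they can differ.
; An ActivateEnemy call exists but never runs.
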(event `self.ReceiveBeginPlay`
  (set `self.RemainingDifficulty` (`self.LevelDifficulty`))
  (`self.SpawnEnemies`))

(event `SpawnEnemies`
  (bind _availableenemies (`self.AvailableEnemies`))
  (bind _returnvalue (`KismetArrayLibrary.Array_Length` _availableenemies))
  (bind (_enemyclass _cost) (break `/Game/enemy/Spawner/ST_EnemySpawnData` (`|GetArrayItem` (`self.AvailableEnemies`) (`KismetMathLibrary.RandomIntegerInRange` 0 (- _returnvalue 1)))))
  (while (> (`self.RemainingDifficulty`) 0)
    (for _array_element (`self.EnemyPool`)
      (if (<= (`.Cost_5_65D0BC05445EF84F2EAFD2A993DA336B` (break `/Game/enemy/Spawner/ST_EnemySpawnData` _array_element)) (`self.RemainingDifficulty`))
        (`KismetArrayLibrary.Array_Add` _availableenemies _array_element)
        (if (== _returnvalue 0)
          (break)
          (else
            (`|SpawnActorFromClass` _enemyclass (`KismetMathLibrary.Conv_VectorToTransform` (`self.K2_GetActorLocation` (`KismetArrayLibrary.Array_Random` (`self.SpawnPoints`)))) "Undefined" "MultiplyWithRoot" null null)
            (set `self.RemainingDifficulty` (- (`self.RemainingDifficulty`) _cost))))))))

(fn `UserConstructionScript`)